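; BP_Baterías is a battery pickup that recharges the first-person character's battery level.
; When the player character overlaps its capsule, it adds BatteryAmount to the character's Nivelbateria, clamped to MáximaBateria, and then destroys itself.
; If the battery is already full, the pickup stays in the world.
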(event `self.Capsule.OnComponentBeginOverlap`
  (params (OverlappedComponent :type "PrimitiveComponent Object Reference") (OtherActor :type "Actor Object Reference") (OtherComp :type "PrimitiveComponent Object Reference") (OtherBodyIndex :type Integer) (bFromSweep :type Boolean) (SweepResult :type "HitResult Structure (by ref)"))
  (bind _asbp_first_person_character (cast `/Game/FirstPerson/Blueprints/BP_FirstPersonCharacter` OtherActor))
  (bind _output_get (set `self.As BP First Person Character` _asbp_first_person_character))
  (bind _nivelbateria (`/Game/FirstPerson/Blueprints/BP_FirstPersonCharacter.Nivelbateria` _output_get))
  (bind `_máximabateria` (`/Game/FirstPerson/Blueprints/BP_FirstPersonCharacter.MáximaBateria` _output_get))
  (if (< _nivelbateria `_máximabateria`)
    (set `/Game/FirstPerson/Blueprints/BP_FirstPersonCharacter.Nivelbateria` (`KismetMathLibrary.FClamp` (+ _nivelbateria (`self.BatteryAmount`)) 0.0 `_máximabateria`) (`self.As BP First Person Character`))
    (`self.K2_DestroyActor`)))

(fn `UserConstructionScript`)