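; BP_Trampilla is an interactable trapdoor that slides when the player presses Interact nearby.
; Its Efe overlap toggles input for BP_FirstPersonCharacter, and both entering and leaving add a new Dialogopuerta widget to the viewport.
; Interact plays a Timeline that lerps the root's relative X location.
; The game mode's CollectableLeft check has empty branches, so it does not gate the movement.
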(event `self.efe.OnComponentBeginOverlap`
  (params (OverlappedComponent :type "PrimitiveComponent Object Reference") (OtherActor :type "Actor Object Reference") (OtherComp :type "PrimitiveComponent Object Reference") (OtherBodyIndex :type Integer) (bFromSweep :type Boolean) (SweepResult :type "HitResult Structure (by ref)"))
  (cast `/Game/FirstPerson/Blueprints/BP_FirstPersonCharacter` OtherActor)
  (`self.EnableInput` (`GameplayStatics.GetPlayerController` 0))
  (bind _returnvalue (`|CreateWidget` "/Game/Dialogos/WB/Dialogopuerta.Dialogopuerta_C" :!label _label))
  (`UserWidget.AddToViewport` _returnvalue 0)
  (`/Engine/EditorBlueprintResources/StandardMacros.DoOnce` false))

(event `self.efe.OnComponentEndOverlap`
  (params (OverlappedComponent :type "PrimitiveComponent Object Reference") (OtherActor :type "Actor Object Reference") (OtherComp :type "PrimitiveComponent Object Reference") (OtherBodyIndex :type Integer))
  (cast `/Game/FirstPerson/Blueprints/BP_FirstPersonCharacter` OtherActor)
  (`self.DisableInput` (`GameplayStatics.GetPlayerController` 0))
  (goto _label))

(event `InputAction|Interact`
  (params (Key :type "Key Structure"))
  (:`Pressed`
    (bind _asbp_first_person_game_mode (cast `/Game/FirstPerson/Blueprints/BP_FirstPersonGameMode` (`GameplayStatics.GetGameMode`)))
    (if (== (`/Game/FirstPerson/Blueprints/BP_FirstPersonGameMode.Collectable Left` _asbp_first_person_game_mode) 0)
      (bind (_direction _newtrack_0) (`Timeline|Timeline` :!label _label_2)
        (:`Update`
          _)
        (:`Finished`
          _))
      (`SceneComponent.K2_SetRelativeLocation` (`self.DefaultSceneRoot`) (`KismetMathLibrary.MakeVector` (`KismetMathLibrary.Lerp` 0.0 90.0 _newtrack_0)) false false)
      (else
        (goto _label_2)))))

(fn `UserConstructionScript`)